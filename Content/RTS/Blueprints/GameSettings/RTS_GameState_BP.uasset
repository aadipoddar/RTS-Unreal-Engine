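; RTS game state that runs the in-game clock and calendar at an adjustable game speed.
; Each tick advances game time, derives clock and date values with month and year rollover, and pushes them to the HUD through the player controller.
; When a day passes, it finds every RTS unit and runs its birthday check.
; Speed updates scale the default speed by a multiplier and broadcast the result.
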(event EventBeginPlay
  (Utilities|FlowControl|Sequence
    (:then_0
      (Utilities|ReferenceCast))
    (:then_1
      ;[1 1 1] Set Default Game Clock and Calender
      (Variables|GameSpeedSettings|SetGame%20Time (+ (Math|Conversions|ToFloat(Integer) (Variables|Clock|GetHours)) (/ (Math|Conversions|ToFloat(Integer) (Variables|Clock|GetMinutes)) 6e+01) (/ (Math|Conversions|ToFloat(Integer) (Variables|Clock|GetHours)) 3.6e+03)))
      (Variables|Calender|SetGame%20Date (Utilities|Array|MakeArray (Variables|Calender|GetDay) (Variables|Calender|GetMonth) (Variables|Calender|GetYear))))
    (:then_2
      ;[1 1 1] Set Default Game Speed
      (Variables|GameSpeedSettings|SetGameSpeed (Variables|GameSpeedSettings|GetDefaultGameSpeed)))))

(event EventTick
  (params (DeltaSeconds :type Float%20%28single-precision%29))
  ;[1 1 1] Update Game Clock and Calender
  (Variables|GameSpeedSettings|SetGame%20Time (.GameTime (CallFunction|SetGameTime DeltaSeconds (Variables|GameSpeedSettings|GetGameSpeed) (Variables|GameSpeedSettings|GetGame%20Time))))
  (Variables|Calender|SetDay%20Counter (.DayCount (CallFunction|SetGameTime DeltaSeconds (Variables|GameSpeedSettings|GetGameSpeed) (Variables|GameSpeedSettings|GetGame%20Time))))
  (CallFunction|SetClock)
  (CallFunction|SetCalender)
  (if (== (.DayCount (CallFunction|SetGameTime DeltaSeconds (Variables|GameSpeedSettings|GetGameSpeed) (Variables|GameSpeedSettings|GetGame%20Time))) 1)
    (bind _units_out (CallFunction|GetAllUnits))
    (for _array_element _units_out
      (Default|BirthdayCheck _array_element))))

(event EventUpdateGameSpeed
  (params (SpeedMultiplier :type Float%20%28single-precision%29))
  ;[1 1 1] Update Game Speed
  (bind _output_get (Variables|GameSpeedSettings|SetSpeedMultiplier SpeedMultiplier))
  (bind _output_get_2 (Variables|GameSpeedSettings|SetGameSpeed (* _output_get (Variables|GameSpeedSettings|GetDefaultGameSpeed))))
  (Default|CallGameSpeedControl _output_get_2))

(fn ConstructionScript)

(fn SetClock
  (bind _game_time (Variables|GameSpeedSettings|GetGame%20Time))
  (bind _returnvalue (* _game_time 3.6e+03))
  (bind (_remainder _returnvalue_2) (Math|Float|Division(WholeandRemainder) _returnvalue 6e+01))
  (bind _returnvalue_3 (Math|Conversions|ToFloat(Integer) _returnvalue_2))
  (bind (_remainder_2 _returnvalue_4) (Math|Float|Division(WholeandRemainder) _returnvalue_3 6e+01))
  (Variables|Clock|SetSeconds (Math|Float|Floor _remainder))
  (Variables|Clock|SetMinutes (Math|Float|Floor _remainder_2))
  (Variables|Clock|SetHours (Math|Float|Floor (.Remainder (Math|Float|Division(WholeandRemainder) (Math|Conversions|ToFloat(Integer) _returnvalue_4) 24.0))))
  (bind _output_get (Variables|Calender|SetGame%20Date (Utilities|Array|MakeArray (Variables|Clock|GetSeconds) (Variables|Clock|GetMinutes) (Variables|Clock|GetHours))))
  (Class|RTSGameTimeIF|SetGameClock(Message) (Variables|/Game/RTS/Blueprints/Player/RTS_PlayerController_BP.RTS_PlayerController_BP_C|GetHUD%20Game%20Time%20Ref (Variables|References|GetControllerRef)) _output_get))

(fn SetCalender
  (bind _output_get (Variables|Calender|SetDay (+ (Variables|Calender|GetDay) (Variables|Calender|GetDay%20Counter))))
  (if (> _output_get (Class|KismetMathLibrary|DaysinMonth (Variables|Calender|GetYear) (Variables|Calender|GetMonth)))
    (Variables|Calender|SetDay 1)
    (Variables|Calender|SetMonth (+ (Variables|Calender|GetMonth) 1)))
  (if (> (Variables|Calender|GetMonth) 12)
    (Variables|Calender|SetMonth 1)
    (Variables|Calender|SetYear (+ (Variables|Calender|GetYear) 1)))
  (bind _output_get_2 (Variables|Calender|SetGame%20Date (Utilities|Array|MakeArray (Variables|Calender|GetDay) (Variables|Calender|GetMonth) (Variables|Calender|GetYear))))
  (Class|RTSGameTimeIF|SetGameCalender(Message) (Variables|/Game/RTS/Blueprints/Player/RTS_PlayerController_BP.RTS_PlayerController_BP_C|GetHUD%20Game%20Time%20Ref (Variables|References|GetControllerRef)) _output_get_2))

(fn GetGameSpeed
  (return (Variables|GameSpeedSettings|GetGameSpeed)))

(fn GetAllUnits
  (bind _outactors (Actor|GetAllActorsOfClass "/Game/RTS/Units/RTS_UnitMaster.RTS_UnitMaster_C"))
  (bind _output_get (Variables|Default|SetList%20Of%20Units _outactors))
  (return _output_get))

(fn SetGameCalender
  (params (Game%20Date :type Array%20of%20Integers))
  (return false))

(fn SetGameClock
  (params (GameTime :type Array%20of%20Integers))
  (return false))