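; Sun rotation Blueprint for the RTS that turns the sun actor over time according to game speed.
; On BeginPlay it reads the speed from the RTS game state and binds to its speed-control event.
; Each tick SetGameTime derives game time from delta time and speed, which is scaled into a local pitch rotation on the sun.
; The sky sphere then updates its sun direction to match.
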(event Custom|Get%20Game%20Speed
  (params (Game%20Speed :type Float%20%28single-precision%29))
  (Variables|Time|SetGame%20Speed Game%20Speed))

(event EventBeginPlay
  (Variables|References|SetGame%20State%20Ref (.AsRTS%20Game%20State%20BP (Utilities|Casting|CastToRTS_GameState_BP (Game|GetGameState))))
  (EventDispatchers|BindEventtoGameSpeedControl (Variables|References|GetGame%20State%20Ref) (EventDispatchers|CreateEvent :!event Custom|Get%20Game%20Speed))
  (bind _game_speed (Default|GetGameSpeed (Variables|References|GetGame%20State%20Ref)))
  (Variables|Time|SetGame%20Speed _game_speed))

(event EventTick
  (params (DeltaSeconds :type Float%20%28single-precision%29))
  (Transformation|AddActorLocalRotation (Variables|References|GetSun%20Ref) (Math|Rotator|MakeRotator 0.0 (* (/ (/ (.GameTime (CallFunction|SetGameTime DeltaSeconds (Variables|Time|GetGame%20Speed) (Variables|Time|GetGame%20Time))) 1.5) 6.0) 9e+01) 0.0) false false)
  (Default|UpdateSunDirection (Variables|References|GetSky%20Sphere%20Ref)))

(fn ConstructionScript)