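; RTS HUD that provides drag-box (marquee) selection of units and ground vehicles.
; Input start clears the previous selection and anchors the box at the mouse, and hold moves the far corner.
; While dragging, DrawHUD draws the rectangle and gathers both classes with GetActorsInSelectionRectangle.
; Release flags those actors as selected, shows their decals and passes both lists to the player controller.
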(event Custom|Draw%20Marquee
  (bind _clicked_location (Variables|MarqueeVariables|GetClicked%20Location))
  (bind _holding_location (Variables|MarqueeVariables|GetHolding%20Location))
  (bind _clicked_location_2 (Variables|MarqueeVariables|GetClicked%20Location))
  (bind _holding_location_2 (Variables|MarqueeVariables|GetHolding%20Location))
  (bind (_x _y) (Math|Vector2D|BreakVector2D _clicked_location_2))
  (bind _returnvalue (- _holding_location_2 _clicked_location_2))
  (bind (_x_2 _y_2) (Math|Vector2D|BreakVector2D _clicked_location))
  (bind (_x_3 _y_3) (Math|Vector2D|BreakVector2D _holding_location))
  (bind (_x_4 _y_4) (Math|Vector2D|BreakVector2D _returnvalue))
  (HUD|DrawRect "(R=0.000000,G=0.000000,B=0.000000,A=0.000000)" _x_2 _y_2 0.0 0.0)
  (HUD|DrawRect "(R=0.000000,G=0.000000,B=0.000000,A=0.000000)" _x_3 _y_3 0.0 0.0)
  (HUD|DrawRect "(R=0.091000,G=0.536000,B=0.761000,A=0.600000)" _x _y _x_4 _y_4))

(event EventBeginPlay
  (Variables|References|SetController%20Ref (.AsRTS%20Player%20Controller%20BP (Utilities|Casting|CastToRTS_PlayerController_BP (Game|GetPlayerController 0)))))

(event EventOnInputStart
  (bind _controller_ref (Variables|References|GetController%20Ref))
  (bind (_locationx _locationy) (Game|Player|GetMousePosition _controller_ref))
  (if (or (>= (Utilities|Array|LastIndex (Variables|Units|GetSelected%20Units)) 0) (>= (Utilities|Array|LastIndex (Variables|Units|GetSelected%20Ground%20Vehicles)) 0))
    (Utilities|FlowControl|Sequence
      (:then_0
        (CallFunction|ClearSelectedUnits))
      (:then_1
        (CallFunction|ClearVehicles))
      (:then_2
        (Default|SetSelectedUnits (Variables|References|GetController%20Ref) (Variables|Units|GetSelected%20Units) (Variables|Units|GetSelected%20Ground%20Vehicles))
        (bind _output_get (Variables|MarqueeVariables|SetClicked%20Location (Math|Vector2D|MakeVector2D _locationx _locationy) :!label _label))
        (Variables|MarqueeVariables|SetHolding%20Location _output_get)
        (Variables|Bool|SetIs%20Drawing true)))
    (else
      (goto _label))))

(event EventOnInputRelease
  (params (Hold%20Time :type Float%20%28single-precision%29))
  (Variables|Bool|SetIs%20Drawing false)
  (CallFunction|SetUnits)
  (CallFunction|SetVehicles)
  (Default|SetSelectedUnits (Variables|References|GetController%20Ref) (Variables|Units|GetSelected%20Units) (Variables|Units|GetSelected%20Ground%20Vehicles)))

(event EventDrawHUD
  (params (SizeX :type Integer) (SizeY :type Integer))
  (if (Variables|Bool|GetIs%20Drawing)
    (Utilities|FlowControl|Sequence
      (:then_0
        (CallFunction|DrawMarquee))
      (:then_1
        (Variables|Units|SetUnits%20in%20Selection%20Area (Class|HUD|GetActorsinSelectionRectangle "/Game/RTS/Units/RTS_UnitMaster.RTS_UnitMaster_C" (Variables|MarqueeVariables|GetClicked%20Location) (Variables|MarqueeVariables|GetHolding%20Location) true false)))
      (:then_2
        (Variables|Units|SetGround%20Vehicles%20In%20Selection%20Area (Class|HUD|GetActorsinSelectionRectangle "/Game/RTS/Units/GroundVehicles/RTS_GroundVehicleMaster.RTS_GroundVehicleMaster_C" (Variables|MarqueeVariables|GetClicked%20Location) (Variables|MarqueeVariables|GetHolding%20Location) true false))))))

(event EventOnInputHold
  (bind _controller_ref (Variables|References|GetController%20Ref))
  (bind (_locationx _locationy) (Game|Player|GetMousePosition _controller_ref))
  (Variables|MarqueeVariables|SetHolding%20Location (Math|Vector2D|MakeVector2D _locationx _locationy)))

(fn ConstructionScript)

(fn ClearSelectedUnits
  (for _array_element (Variables|Units|GetSelected%20Units)
    (Default|SetDeselectedDecal _array_element)
    (Variables|/Game/RTS/Units/RTS_UnitMaster.RTS_UnitMaster_C|SetIs%20Selected _array_element false)
    (Variables|/Game/RTS/Blueprints/Player/RTS_PlayerController_BP.RTS_PlayerController_BP_C|SetIs%20Unit%20Selected (Variables|References|GetController%20Ref) false))
  (Utilities|Array|Clear (Variables|Units|GetSelected%20Units)))

(fn ClearVehicles
  (for _array_element (Variables|Units|GetSelected%20Ground%20Vehicles)
    (Default|SetDeselectedDecal _array_element)
    (Variables|/Game/RTS/Units/GroundVehicles/RTS_GroundVehicleMaster.RTS_GroundVehicleMaster_C|SetIs%20Selected _array_element false)
    (Variables|/Game/RTS/Blueprints/Player/RTS_PlayerController_BP.RTS_PlayerController_BP_C|SetIs%20Unit%20Selected (Variables|References|GetController%20Ref) false))
  (Utilities|Array|Clear (Variables|Units|GetSelected%20Ground%20Vehicles)))

(fn SetUnits
  (for _array_element (Variables|Units|GetUnits%20in%20Selection%20Area)
    (if (Utilities|ClassIsChildOf (Utilities|GetClass _array_element) "/Game/RTS/Units/RTS_UnitMaster.RTS_UnitMaster_C")
      (bind _asrts_unit_master (Utilities|Casting|CastToRTS_UnitMaster _array_element))
      (Variables|Units|SetSelected%20Unit _asrts_unit_master)
      (Utilities|FlowControl|Sequence
        (:then_0
          (Utilities|Array|AddUnique (Variables|Units|GetSelected%20Units) (Variables|Units|GetSelected%20Unit)))
        (:then_1
          (for _array_element_2 (Variables|Units|GetSelected%20Units)
            (Default|SetSelectedDecal _array_element_2)
            (Variables|/Game/RTS/Units/RTS_UnitMaster.RTS_UnitMaster_C|SetIs%20Selected _array_element_2 true)))))))

(fn SetVehicles
  (for _array_element (Variables|Units|GetGround%20Vehicles%20In%20Selection%20Area)
    (if (Utilities|ClassIsChildOf (Utilities|GetClass _array_element) "/Game/RTS/Units/GroundVehicles/RTS_GroundVehicleMaster.RTS_GroundVehicleMaster_C")
      (bind _asrts_ground_vehicle_master (Utilities|Casting|CastToRTS_GroundVehicleMaster _array_element))
      (Variables|Units|SetSelected%20Ground%20Vehicle _asrts_ground_vehicle_master)
      (Utilities|FlowControl|Sequence
        (:then_0
          (Utilities|Array|AddUnique (Variables|Units|GetSelected%20Ground%20Vehicles) (Variables|Units|GetSelected%20Ground%20Vehicle)))
        (:then_1
          (for _array_element_2 (Variables|Units|GetSelected%20Ground%20Vehicles)
            (Default|SetSelectedDecal _array_element_2)
            (Variables|/Game/RTS/Units/GroundVehicles/RTS_GroundVehicleMaster.RTS_GroundVehicleMaster_C|SetIs%20Selected _array_element_2 true)))))))