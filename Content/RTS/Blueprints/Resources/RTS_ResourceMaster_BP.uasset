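; Base resource Blueprint for the RTS that sets up a resource's amount and appearance in its Construction Script.
; A resource level, optionally randomized, selects a multiplier that scales the base amount into the current resources.
; Optional flags randomize the mesh's scale independently on each axis within min and max bounds, and its yaw rotation, to vary placed instances.
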(fn ConstructionScript
  (bind _min_mesh_size (Variables|ResourceSize|GetMin%20Mesh%20Size))
  (bind _max_mesh_size (Variables|ResourceSize|GetMax%20Mesh%20Size))
  (bind _returnvalue (Math|Random|RandomFloatinRange _min_mesh_size _max_mesh_size))
  (if (Variables|Bool|GetIs%20Random%20Level)
    (bind _output_get (Variables|References|SetResource%20Level%20Enum%20Ref (Utilities|Enum|ByteToEnumResourceLevelEnum (Math|Conversions|ToByte(Integer) (Math|Random|RandomIntegerinRange 1 6))))))
  (switch Utilities|FlowControl|Switch|SwitchonResourceLevelEnum _output_get
    (:NewEnumerator1
      (Variables|References|SetResource%20Modifier 1.0))
    (:NewEnumerator2
      (Variables|References|SetResource%20Modifier 1.2))
    (:NewEnumerator3
      (Variables|References|SetResource%20Modifier 1.4))
    (:NewEnumerator4
      (Variables|References|SetResource%20Modifier 1.6))
    (:NewEnumerator5
      (Variables|References|SetResource%20Modifier 1.8))
    (:NewEnumerator6
      (Variables|References|SetResource%20Modifier 2.0)))
  (Variables|ResorceValue|SetCurrent%20Resources (* (Variables|ResorceValue|GetBase%20Resource%20Amount) (Variables|References|GetResource%20Modifier)))
  (if (Variables|Bool|GetIs%20Random%20Size)
    (Transformation|SetWorldScale3D (Variables|Default|GetResourceMesh) (Math|Vector|MakeVector _returnvalue _returnvalue _returnvalue)))
  (if (Variables|Bool|GetIs%20Random%20Rotated)
    (Transformation|SetWorldRotation (Variables|Default|GetResourceMesh) (Math|Rotator|MakeRotator 0.0 0.0 (Math|Random|RandomFloatinRange 0.0 3.6e+02)) false false)))