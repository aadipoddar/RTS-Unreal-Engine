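; RTS spawn volume that scatters resource actors over the landscape within its bounds, at begin play and optionally on a looping timer up to a total cap.
; Each spawn box-traces at a random XY point and only places the resource on a Landscape hit, though misses still count toward the cap.
; RespawnTime follows game speed and/or a custom value, but the timer takes it once, starts only with begin-play spawning, and skips while paused.
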(event Custom|Spawn%20Resources%20On%20Timer
  (if (not (Variables|/Game/RTS/Blueprints/Widgets/GameTime_HUD.GameTime_HUD_C|GetIs%20Paused (Variables|/Game/RTS/Blueprints/Player/RTS_PlayerController_BP.RTS_PlayerController_BP_C|GetHUD%20Game%20Time%20Ref (Variables|References|GetPlayer%20Controller%20Ref))))
    (if (and (Variables|Bool|GetIs%20Spawn%20On%20Timer) (< (Variables|ResourceSettings|GetTotal%20Number%20Spawned) (Variables|ResourceSettings|GetMax%20Resources%20Spawned)))
      (CallFunction|SpawnResource (Variables|References|GetResource%20Ref) (Variables|ResourceSettings|GetNum%20Of%20Resources%20Spawn))
      (Variables|ResourceSettings|SetTotal%20Number%20Spawned (+ (Variables|ResourceSettings|GetNum%20Of%20Resources%20Spawn) (Variables|ResourceSettings|GetTotal%20Number%20Spawned))))))

(event Custom|Get%20Game%20Speed
  (params (Game%20Speed :type Float%20%28single-precision%29))
  (Variables|ResourceSettings|SetGame%20Speed Game%20Speed))

(event EventBeginPlay
  (Utilities|FlowControl|Sequence
    (:then_0
      (Utilities|ReferenceCasts))
    (:then_1
      (EventDispatchers|BindEventtoGameSpeedControl (Variables|References|GetGame%20State%20Ref) (EventDispatchers|CreateEvent :!event Custom|Get%20Game%20Speed))
      (bind _game_speed (Default|GetGameSpeed (Variables|References|GetGame%20State%20Ref)))
      (Variables|ResourceSettings|SetGame%20Speed _game_speed)
      (CallFunction|SetRespawnTimer))
    (:then_2
      (if (Variables|Bool|GetIs%20Spawn%20On%20Begin%20Play)
        (CallFunction|SpawnResource (Variables|References|GetResource%20Ref) (Variables|ResourceSettings|GetNum%20Of%20Resources%20Spawn))
        (Variables|ResourceSettings|SetTotal%20Number%20Spawned (+ (Variables|ResourceSettings|GetNum%20Of%20Resources%20Spawn) (Variables|ResourceSettings|GetTotal%20Number%20Spawned)))
        (if (and (Variables|Bool|GetIs%20Spawn%20On%20Timer) (< (Variables|ResourceSettings|GetTotal%20Number%20Spawned) (Variables|ResourceSettings|GetMax%20Resources%20Spawned)))
          (Utilities|Time|SetTimerbyEvent (EventDispatchers|CreateEvent :!event Custom|Spawn%20Resources%20On%20Timer) (Variables|ResourceSettings|GetRespawn%20Time) true))))))

(event EventTick
  (params (DeltaSeconds :type Float%20%28single-precision%29))
  (CallFunction|SetRespawnTimer))

(fn ConstructionScript)

(fn SpawnResource
  (params (Resource :type RTS%20Resource%20Master%20BP%20Class%20Reference) (Spawn%20Amount :type Integer))
  (bind (_origin _boxextent) (Collision|GetActorBounds false false))
  (bind _z (Math|Vector|BreakVector _origin))
  (bind (_x _y) (Math|Vector|BreakVector _boxextent))
  (bind _returnvalue (* _y 2.0))
  (bind _returnvalue_2 (* _x 2.0))
  (bind _returnvalue_3 (- _x _returnvalue_2))
  (bind _returnvalue_4 (- _y _returnvalue))
  (bind _returnvalue_5 (Math|Random|RandomFloatinRange _returnvalue_3 _x))
  (bind _returnvalue_6 (Math|Random|RandomFloatinRange _returnvalue_4 _y))
  (bind _returnvalue_7 (Math|Vector|MakeVector _returnvalue_5 _returnvalue_6 _z))
  (bind _returnvalue_8 (+ _origin _returnvalue_7))
  (LocalVariables|SetResource%20Ref%20Local Resource)
  (LocalVariables|SetSpawn%20Amount%20Local Spawn%20Amount)
  (for _index (range 0 (LocalVariables|GetSpawn%20Amount%20Local))
    (bind _outhit (Collision|BoxTraceByChannel (+ _returnvalue_8 "0, 0,200.000000") "0, 0, 0" (- _returnvalue_8 (Math|Vector|MakeVector 0.0 0.0 2e+02)) "0, 0, 0" "TraceTypeQuery1" false 0 "None"))
    (if (== (Utilities|GetClass (.HitActor (Collision|BreakHitResult _outhit))) "/Script/Landscape.Landscape")
      (Game|SpawnActorfromClass (LocalVariables|GetResource%20Ref%20Local) (Math|Conversions|ToTransform(Vector) (.Location (Collision|BreakHitResult _outhit))) "Undefined" 0 0))))

(fn SetRespawnTimer
  (switch Utilities|FlowControl|Switch|SwitchonRespawnTimerEnum (Variables|References|GetTime%20Setting)
    (:NewEnumerator1
      (Variables|ResourceSettings|SetRespawn%20Time 0.0))
    (:NewEnumerator2
      (Variables|ResourceSettings|SetRespawn%20Time (Variables|ResourceSettings|GetGame%20Speed)))
    (:NewEnumerator3
      (Variables|ResourceSettings|SetRespawn%20Time (Variables|ResourceSettings|GetUser%20Respawn%20Timer)))
    (:NewEnumerator4
      (Variables|ResourceSettings|SetRespawn%20Time (* (Variables|ResourceSettings|GetUser%20Respawn%20Timer) (Variables|ResourceSettings|GetGame%20Speed)))))
  (return (Variables|ResourceSettings|GetRespawn%20Time)))