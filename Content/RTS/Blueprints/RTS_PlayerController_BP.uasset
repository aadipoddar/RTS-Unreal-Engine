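; RTS player controller that drives the strategy camera pawn from movement axis input.
; On BeginPlay it casts the player pawn to RTS_CameraPawn_BP and caches the reference.
; MoveForward and MoveRight axes feed world-space X and Y vectors into that pawn's FloatingPawnMovement, so panning ignores camera facing.
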(event EventBeginPlay
  (Utilities|ReferenceCast) ; Should Always be First
)

(event Input|AxisEvents|InputAxisMoveForward
  (params (AxisValue :type Float%20%28single-precision%29))
  (Class|PawnMovementComponent|AddInputVector (Variables|/Game/RTS/Blueprints/RTS_CameraPawn_BP.RTS_CameraPawn_BP_C|GetFloatingPawnMovement (Variables|References|GetCameraPawnRef)) (Math|Vector|MakeVector AxisValue 0.0 0.0) false))

(event Input|AxisEvents|InputAxisMoveRight
  (params (AxisValue :type Float%20%28single-precision%29))
  (Class|PawnMovementComponent|AddInputVector (Variables|/Game/RTS/Blueprints/RTS_CameraPawn_BP.RTS_CameraPawn_BP_C|GetFloatingPawnMovement (Variables|References|GetCameraPawnRef)) (Math|Vector|MakeVector 0.0 AxisValue 0.0) false))

(fn ConstructionScript)